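; Gun tower for DroidDefense that shoots at the in-range unit closest to the base.
; Each tick it gathers "Unit" actors within range and sorts them by distance to the "Base" actor via the ObjectCompare comparator.
; It turns the turret top and gun toward the first target, then spawns a BP_Bullet carrying its damage when MCanFire is set.
; Firing clears that flag; nothing in these graphs resets it or counts down the fire timer.
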(event EventBeginPlay
  (Variables|Default|Setm_Range 8e+02)
  (Variables|Default|Setm_FireTimerMax 1.25)
  (Variables|Default|Setm_Damage 1e+01)
  (bind _outactors (Actor|GetAllActorswithTag "Base"))
  (Variables|Default|SetBase (Utilities|Array|Get(acopy) _outactors))
  (Variables|Default|Setm_Cost 10))

(event EventTick
  (params (DeltaSeconds :type Float%20%28single-precision%29))
  (bind _validtargets (Variables|Default|GetValidTargets))
  (bind _gun (Variables|Default|GetGun))
  (bind _guntop (Variables|Default|GetGunTop))
  (bind _item (Utilities|Array|Get(acopy) _validtargets))
  (bind _returnvalue (Transformation|GetWorldLocation _guntop))
  (bind _returnvalue_2 (Transformation|GetWorldTransform _gun))
  (bind _returnvalue_3 (Transformation|GetActorLocation _item))
  (bind _returnvalue_4 (Math|Rotator|FindLookatRotation _returnvalue _returnvalue_3))
  (bind _returnvalue_5 (- (.yaw _returnvalue_4) 9e+01))
  (Utilities|Array|Clear (Variables|Default|GetValidTargets))
  (bind _outactors (Actor|GetAllActorswithTag "Unit"))
  (for _array_element _outactors
    ;[1 1 1] Find the units that can be shoot at
    (if (<= (Math|Vector|VectorLength (- (Transformation|GetActorLocation _array_element) (Transformation|GetWorldLocation (Variables|Default|GetBox)))) (Variables|Default|Getm_Range))
      (Utilities|Array|Add (Variables|Default|GetValidTargets) _array_element)))
  ;[1 1 1] Only proced if the array has stuff in it and is sorted
  (if (> (Utilities|Array|Length (Variables|Default|GetValidTargets)) 0)
    (Class|LowEntryExtendedStandardLibrary|SortObjectArrayDirectly (Variables|Default|GetValidTargets) (EventDispatchers|CreateEvent :!event ObjectCompare) false)
    ;[1 1 1] Make the top of the turret face the enemy closest to the goal
    (Transformation|SetWorldRotation (Variables|Default|GetGunTop) (Math|Rotator|MakeRotator 0.0 0.0 _returnvalue_5) false false)
    (Transformation|SetWorldRotation (Variables|Default|GetGun) (Math|Rotator|MakeRotator (.roll _returnvalue_4) (.pitch _returnvalue_4) _returnvalue_5) false false)
    ;[1 1 1] If possible fire a bullet
    (if (Variables|Default|Getm_CanFire)
      (Game|SpawnActorfromClass "/Game/DroidDefense/Ammo/BP_Bullet.BP_Bullet_C" (Math|Transform|MakeTransform (Math|Vector|MakeVector (.x (.location _returnvalue_2)) (+ (.y (.location _returnvalue_2)) 75.0) (.z (.location _returnvalue_2))) (.rotation _returnvalue_2) "1.000000,1.000000,1.000000") "Undefined" 0 (Variables|Default|Getm_Damage) 0)
      (Variables|Default|Setm_CanFire false))))

(fn ConstructionScript)

(fn ObjectCompare
  (params (Obj1 :type Object%20Object%20Reference) (Obj2 :type Object%20Object%20Reference))
  (bind _base (Variables|Default|GetBase))
  (bind _returnvalue (Transformation|GetActorLocation _base))
  (bind _asactor (Utilities|Casting|CastToActor Obj1)
    (:then
      (bind _asactor_2 (Utilities|Casting|CastToActor Obj2)
        (:then
          (return (<= (Math|Vector|VectorLength (- (Transformation|GetActorLocation _asactor) _returnvalue)) (Math|Vector|VectorLength (- (Transformation|GetActorLocation _asactor_2) _returnvalue)))))
        (:CastFailed
          _)))
    (:CastFailed
      _))
  (return false))