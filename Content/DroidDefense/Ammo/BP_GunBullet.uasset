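; BP_GunBullet is a Droid Defense gun bullet that damages actors tagged Base.
; On overlap it sends its Damage to a Base actor through DealDamageMessage and destroys itself; Floor actors destroy it without damage.
; Tick counts Life down and destroys the bullet below zero.
; The graph's physics and rotation nodes are disconnected, so no active logic here moves it.
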(event EventBeginPlay)

(event Collision|EventActorBeginOverlap
  (params (OtherActor :type Actor%20Object%20Reference))
  (if (Actor|ActorHasTag OtherActor "Base")
    (Class|BPIDamagable|DealDamage(Message) OtherActor (Variables|Default|GetDamage))
    (Actor|DestroyActor :!label _label)
    (elif (Actor|ActorHasTag OtherActor "Floor")
      (goto _label))))

(event EventTick
  (params (DeltaSeconds :type Float%20%28single-precision%29))
  (bind _output_get (Variables|Default|SetLife (- (Variables|Default|GetLife) DeltaSeconds)))
  (if (< _output_get 0.0)
    (Actor|DestroyActor)))

(fn ConstructionScript)