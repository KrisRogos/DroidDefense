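; Player controller for DroidDefense that handles drag-and-drop placement of gun towers on a grid, plus quitting the app.
; A left click spends 10 of the player character's parts to spawn a tower at the snapped cursor location, and Tick drags it across tiles the map manager approves.
; Release registers it with the map, falling back to its last position or destroying it without refund.
; Touch input only sets flags.
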(event EventBeginPlay
  (bind _outactors (Actor|GetAllActorsOfClass "/Script/DroidDefense.C_MapMngr"))
  (if (== (Utilities|Array|Length _outactors) 1)
    (Variables|Default|SetMap (Utilities|Array|Get(acopy) _outactors))
    (else
      (Class|VisualLoggerKismetLibrary|LogText "No map manager found" "Blueprint Error")
      (Game|QuitGame 0 "Quit"))))

(event EventTick
  (params (DeltaSeconds :type Float%20%28single-precision%29))
  (bind _hitresult (Game|Player|GetHitResultUnderCursorbyChannel "TraceTypeQuery1" true))
  (bind _map (Variables|Default|GetMap))
  (bind (_debug_text _loc_x _loc_y) (Utilities|GetGridCoordinates (.location _hitresult)))
  (if (Variables|Default|GetMouseDown)
    (Utilities|IsValid _map
      (:Is%20Valid
        (bind _returnvalue (Class|CMapMngr|CheckTile _map _loc_x _loc_y))
        (if _returnvalue
          (Transformation|SetActorLocation (Variables|Default|GetNew%20Tower) (.Grid%20Aligned%20Location (Utilities|SnapLocationtoGrid (.location _hitresult))) false false))))))

(event Input|ActionEvents|InputActionClick
  (params (Key :type Key%20Structure :default "AnyKey"))
  (bind _returnvalue (== Key "LeftMouseButton"))
  (bind _hitresult (Game|Player|GetHitResultUnderCursorbyChannel "TraceTypeQuery1" true))
  (:Pressed
    (if _returnvalue
      ;[1 1 1] Only one type of input to be used at any given time
      (Variables|Default|SetMouseDown true)
      (Variables|Default|SetTouchDown false)
      (|Createthetoweratclickedlocation (.location _hitresult) (.hitactor _hitresult))
      (else
        (Variables|Default|SetTouchDown true)
        (Variables|Default|SetMouseDown false))))
  (:Released
    (if _returnvalue
      (Variables|Default|SetMouseDown false)
      (|Placethetoweratfinallocation (.location _hitresult))
      (else
        (Variables|Default|SetTouchDown false)))))

(event Input|ActionEvents|InputActionAddBasicTower
  (params (Key :type Key%20Structure :default "AnyKey")))

(event Input|ActionEvents|InputActionAppClose
  (params (Key :type Key%20Structure :default "AnyKey"))
  (:Pressed
    (Game|QuitGame 0 "Quit")))

(fn ConstructionScript)