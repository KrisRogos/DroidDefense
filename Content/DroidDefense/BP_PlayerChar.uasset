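; Player character for Droid Defense that holds the steam and parts counters and drives the main HUD and win/lose screens.
; On BeginPlay it moves to a stored transform and, if exactly one enemy spawner exists, caches it and creates the HUD.
; Tick polls for steam running out (loss) or all enemy units gone (win), rebuilding the matching end screen every frame while that holds.
; Helper functions add parts and relay the spawner's current wave.
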(event EventBeginPlay
  (bind _newvar_0 (Variables|Default|GetNewVar_0))
  (bind _newvar_1 (Variables|Default|GetNewVar_1))
  (Transformation|SetActorLocationAndRotation _newvar_0 _newvar_1)
  (Transformation|SetWorldLocationAndRotation (Variables|Collision|GetCapsuleComponent) _newvar_0 _newvar_1 false false)
  (bind _outactors (Actor|GetAllActorsOfClass "/Game/DroidDefense/Map/BP_EnemySpawn.BP_EnemySpawn_C"))
  (if (== (Utilities|Array|Length _outactors) 1)
    (Variables|Default|SetEnemyBase (Utilities|Array|Get(acopy) _outactors))
    (bind _returnvalue (UserInterface|CreateWidget "/Game/DroidDefense/HUD/MainHUd.MainHUD_C" (Game|GetPlayerController 0)))
    (UserInterface|Viewport|AddtoViewport _returnvalue 0)
    (Variables|/Game/DroidDefense/HUD/MainHUd.MainHUD_C|SetPlayerRef _returnvalue self)))

(event Collision|EventActorBeginOverlap
  (params (OtherActor :type Actor%20Object%20Reference)))

(event EventTick
  (params (DeltaSeconds :type Float%20%28single-precision%29))
  (if (<= (Variables|Default|GetSteamCounter) 0)
    ;[1 1 1] Lost screen
    (Viewport|RemoveAllWidgets)
    (bind _returnvalue (UserInterface|CreateWidget "/Game/DroidDefense/HUD/GameLost.GameLost_C" (Game|GetPlayerController 0)))
    (UserInterface|Viewport|AddtoViewport _returnvalue 0)
    (Variables|/Game/DroidDefense/HUD/GameLost.GameLost_C|SetPlayerRef _returnvalue self)
    (else
      (bind _gone (Default|AllUnitsGone (Variables|Default|GetEnemyBase)))
      (if _gone
        ;[1 1 1] Win screen
        (Viewport|RemoveAllWidgets)
        (bind _returnvalue_2 (UserInterface|CreateWidget "/Game/DroidDefense/HUD/GameWon.GameWon_C" (Game|GetPlayerController 0)))
        (UserInterface|Viewport|AddtoViewport _returnvalue_2 0)
        (Variables|/Game/DroidDefense/HUD/GameWon.GameWon_C|SetPlayerRef _returnvalue_2 self)))))

(fn ConstructionScript)

(fn AddParts
  (params (Amount :type Integer))
  (Variables|Default|SetPartCounter (+ Amount (Variables|Default|GetPartCounter))))

(fn GetWaveStatus
  (bind _enemybase (Variables|Default|GetEnemyBase))
  (Utilities|IsValid _enemybase
    (:Is%20Valid
      (bind _newparam (Default|GetCurrentWave _enemybase))
      (return _newparam))))