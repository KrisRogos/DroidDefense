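; Droid Defense unit that moves toward a target location, fires gun bullets at it when in range, and awards parts to the player on death.
; The map manager pathfinds to a fixed grid cell; spawned markers display the route and FindPath rebuilds them.
; Movement uses SimpleMoveToLocation independently of those nodes.
; Tick also drives the one-second fire timer, updates the health bar and tilts it toward the player with fixed yaw.
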(event EventBeginPlay
  (bind (_x _y) (Utilities|GetCurrentGridXY))
  (|CallParentFunction)
  (Variables|Default|Setm_TargetX 18)
  (Variables|Default|Setm_TargetY 8)
  (Pawn|SpawnDefaultController)
  (bind _output_get (Variables|Default|Setm_Health 5e+01))
  (Variables|Default|Setm_MaxHealth _output_get)
  (Variables|Default|Setm_PartsDeath 5)
  ;[1 1 1] Get a map reference
  (bind _outactors (Actor|GetAllActorsOfClass "/Script/DroidDefense.C_MapMngr"))
  (if (== (Utilities|Array|Length _outactors) 1)
    ;[1 1 1] Find the path
    (bind _returnvalue (Class|CMapMngr|PathFind (Utilities|Array|Get(acopy) _outactors) _x _y (Variables|Default|Getm_TargetX) (Variables|Default|Getm_TargetY) (Variables|Default|GetNodes)))
    (for _array_element _returnvalue
      (Utilities|SpawnPathObject _array_element))))

(event Collision|EventActorBeginOverlap
  (params (OtherActor :type Actor%20Object%20Reference)))

(event EventTick
  (params (DeltaSeconds :type Float%20%28single-precision%29))
  (bind _returnvalue (Game|GetPlayerCharacter 0))
  (bind _capsulecomponent (Variables|Default|GetCapsuleComponent))
  (bind _uicontainer (Variables|Default|GetUIContainer))
  (bind _m_targetloc (Variables|Default|Getm_TargetLoc))
  (bind _returnvalue_2 (Transformation|GetWorldLocation _uicontainer))
  (bind _returnvalue_3 (Transformation|GetActorLocation _returnvalue))
  (bind _returnvalue_4 (Transformation|GetWorldTransform _capsulecomponent))
  (bind _returnvalue_5 (Math|Rotator|FindLookatRotation (.location _returnvalue_4) _m_targetloc))
  (bind _returnvalue_6 (Math|Rotator|FindLookatRotation _returnvalue_2 _returnvalue_3))
  (Variables|Default|Settimer (+ DeltaSeconds (Variables|Default|Gettimer)))
  (bind _asunit_health (Utilities|Casting|CastToUnitHealth (UserInterface|GetUserWidgetObject (Variables|Default|GetHealthUI))))
  (Progress|SetPercent (Variables|/Game/DroidDefense/HUD/UnitHealth.UnitHealth_C|GetProgressBar_Health _asunit_health) (/ (Variables|Default|Getm_Health) (Variables|Default|Getm_MaxHealth)))
  (Transformation|SetWorldRotation (Variables|Default|GetUIContainer) (Math|Rotator|MakeRotator (.roll _returnvalue_6) (.pitch _returnvalue_6) 1.8e+02) false false)
  (AI|Navigation|SimpleMovetoLocation (Pawn|GetController) (Variables|Default|Getm_TargetLoc))
  (if (and (<= (Math|Vector|VectorLength (- (Transformation|GetActorLocation) (Variables|Default|Getm_TargetLoc))) 5e+02) (>= (Variables|Default|Gettimer) 1.0))
    (Game|SpawnActorfromClass "/Game/DroidDefense/Ammo/BP_GunBullet.BP_GunBullet_C" (Math|Transform|MakeTransform (.location _returnvalue_4) (Math|Rotator|MakeRotator (.roll _returnvalue_5) (.pitch _returnvalue_5) (- (.yaw _returnvalue_5) 9e+01)) "1,1,1") "Undefined" 0 1.2 0)
    (Variables|Default|Settimer 0.0)))

(event EventFindPath
  (bind (_x _y) (Utilities|GetCurrentGridXY))
  ;[1 1 1] Remove nodes from the old array
  (for (_array_element _array_index) (Variables|Default|Getmrp_PathNodes)
    (Actor|DestroyActor _array_element)
    (Utilities|Array|SetArrayElem (Variables|Default|Getmrp_PathNodes) _array_index 0))
  (Utilities|Array|Clear (Variables|Default|Getmrp_PathNodes))
  ;[1 1 1] Get a map reference
  (bind _outactors (Actor|GetAllActorsOfClass "/Script/DroidDefense.C_MapMngr"))
  (if (== (Utilities|Array|Length _outactors) 1)
    ;[1 1 1] Find the path
    (bind _returnvalue (Class|CMapMngr|PathFind (Utilities|Array|Get(acopy) _outactors) _x _y (Variables|Default|Getm_TargetX) (Variables|Default|Getm_TargetY) (Variables|Default|GetNodes)))
    (for _array_element_2 _returnvalue
      (Utilities|SpawnPathObject _array_element_2))))

(event EventDealDamage
  (params (Amount :type Float%20%28single-precision%29))
  (bind _output_get (Variables|Default|Setm_Health (- (Variables|Default|Getm_Health) Amount)))
  (if (<= _output_get 0.0)
    (bind _asbp_player_char (Utilities|Casting|CastToBP_PlayerChar (Game|GetPlayerCharacter 0))
      (:then
        (Default|AddParts _asbp_player_char (Variables|Default|Getm_PartsDeath))
        (Actor|DestroyActor))
      (:CastFailed
        (Actor|DestroyActor)))))

(fn ConstructionScript)