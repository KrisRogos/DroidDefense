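; BP_BasicUnit is a DroidDefense unit that marches on the base, shoots at it, and awards parts to the player when killed.
; FindMyPath asks C_MapMngr for a grid path and spawns BP_ChosenPath actors as waypoints, rebuilt on FindPath.
; Tick updates the player-facing health bar, moves through waypoints with the base as fallback, and fires timed BP_GunBullet shots when the base is in range.
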(event EventBeginPlay
  (|CallParentFunction)
  (Variables|Default|Setm_CurrentNode 0)
  (Variables|Default|Setm_TargetX 8)
  (Variables|Default|Setm_TargetY 17)
  (Pawn|SpawnDefaultController)
  (bind _output_get (Variables|Default|Setm_Health 5e+01))
  (Variables|Default|Setm_MaxHealth _output_get)
  (Variables|Default|Setm_PartsDeath 5)
  (CallFunction|FindMyPath))

(event Collision|EventActorBeginOverlap
  (params (OtherActor :type Actor%20Object%20Reference)))

(event EventTick
  (params (DeltaSeconds :type Float%20%28single-precision%29))
  (bind _returnvalue (Game|GetPlayerCharacter 0))
  (bind _capsulecomponent (Variables|Default|GetCapsuleComponent))
  (bind _uicontainer (Variables|Default|GetUIContainer))
  (bind _m_targetloc (Variables|Default|Getm_TargetLoc))
  (bind _returnvalue_2 (Transformation|GetWorldLocation _uicontainer))
  (bind _returnvalue_3 (Transformation|GetActorLocation _returnvalue))
  (bind _returnvalue_4 (Transformation|GetWorldTransform _capsulecomponent))
  (bind _returnvalue_5 (Math|Rotator|FindLookatRotation (.location _returnvalue_4) _m_targetloc))
  (bind _returnvalue_6 (Math|Rotator|FindLookatRotation _returnvalue_2 _returnvalue_3))
  (Variables|Default|Settimer (+ DeltaSeconds (Variables|Default|Gettimer)))
  (bind _asunit_health (Utilities|Casting|CastToUnitHealth (UserInterface|GetUserWidgetObject (Variables|Default|GetHealthUI))))
  (Progress|SetPercent (Variables|/Game/DroidDefense/HUD/UnitHealth.UnitHealth_C|GetProgressBar_Health _asunit_health) (/ (Variables|Default|Getm_Health) (Variables|Default|Getm_MaxHealth)))
  (Transformation|SetWorldRotation (Variables|Default|GetUIContainer) (Math|Rotator|MakeRotator (.roll _returnvalue_6) (.pitch _returnvalue_6) 1.8e+02) false false)
  (bind _target_loc (CallFunction|GetWaypointLocation))
  (AI|Navigation|SimpleMovetoLocation (Pawn|GetController) _target_loc)
  (if (and (<= (Math|Vector|VectorLength (- (Transformation|GetActorLocation) (Variables|Default|Getm_TargetLoc))) 1e+03) (>= (Variables|Default|Gettimer) 1.0))
    (Game|SpawnActorfromClass "/Game/DroidDefense/Ammo/BP_GunBullet.BP_GunBullet_C" (Math|Transform|MakeTransform (.location _returnvalue_4) (Math|Rotator|MakeRotator (.roll _returnvalue_5) (.pitch _returnvalue_5) (- (.yaw _returnvalue_5) 9e+01)) "1,1,1") "Undefined" 0 (Variables|Default|GetDamge) 0)
    (Variables|Default|Settimer 0.0)))

(event EventFindPath
  (CallFunction|ClearOldPath)
  (CallFunction|FindMyPath))

(event EventDealDamage
  (params (Amount :type Float%20%28single-precision%29))
  (bind _output_get (Variables|Default|Setm_Health (- (Variables|Default|Getm_Health) Amount)))
  (if (<= _output_get 0.0)
    (bind _asbp_player_char (Utilities|Casting|CastToBP_PlayerChar (Game|GetPlayerCharacter 0))
      (:then
        (Default|AddParts _asbp_player_char (Variables|Default|Getm_PartsDeath))
        (CallFunction|ClearOldPath)
        (Actor|DestroyActor))
      (:CastFailed
        (Actor|DestroyActor)))))

(fn ConstructionScript)

(fn GetWaypointLocation
  (bind _mrp_pathnodes (Variables|Default|Getmrp_PathNodes))
  ;[1 1 1] Check distance to current waypoint
  (bind _asbp_chosen_path (Utilities|Casting|CastToBP_ChosenPath (Utilities|Array|Get(acopy) (Variables|Default|Getmrp_PathNodes) (Variables|Default|Getm_CurrentNode)))
    (:then
      (if (< (Math|Vector|VectorLength (- (Transformation|GetWorldLocation (Variables|/Game/DroidDefense/Path_Finder/BP_ChosenPath.BP_ChosenPath_C|GetCube _asbp_chosen_path)) (Transformation|GetWorldLocation (Variables|Character|GetMesh)))) 2.5e+02)
        ;[1 1 1] Select next waypoint
        (bind _result (Math|Integer|IncrementInt (Variables|Default|Getm_CurrentNode))
          (:%20%20
            ;[1 1 1] Go to next waypoint
            (if (< _result (Utilities|Array|Length _mrp_pathnodes))
              (bind _asbp_chosen_path_2 (Utilities|Casting|CastToBP_ChosenPath (Utilities|Array|Get(acopy) _mrp_pathnodes _result))
                (:then
                  (return (Transformation|GetWorldLocation (Variables|/Game/DroidDefense/Path_Finder/BP_ChosenPath.BP_ChosenPath_C|GetCube _asbp_chosen_path_2))) ; Go to current waypoint
                )
                (:CastFailed
                  (return (Variables|Default|Getm_TargetLoc)) ; Error, go to base
                ))
              (else
                (return (Variables|Default|Getm_TargetLoc)) ; Go to the base instead
              ))))
        (else
          (return (Transformation|GetWorldLocation (Variables|/Game/DroidDefense/Path_Finder/BP_ChosenPath.BP_ChosenPath_C|GetCube _asbp_chosen_path))) ; Go to current waypoint
        )))
    (:CastFailed
      (return (Variables|Default|Getm_TargetLoc)) ; Error, go to base
    )))

(fn FindMyPath
  (bind (_x _y) (Utilities|GetCurrentGridXY))
  (Variables|Default|Setm_CurrentNode 0)
  ;[1 1 1] Remove nodes from the old array
  (for (_array_element _array_index) (Variables|Default|Getmrp_PathNodes)
    (Actor|DestroyActor _array_element)
    (Utilities|Array|SetArrayElem (Variables|Default|Getmrp_PathNodes) _array_index 0))
  (Utilities|Array|Clear (Variables|Default|Getmrp_PathNodes))
  (Utilities|Array|Clear (Variables|Default|GetNodes))
  ;[1 1 1] Get a map reference
  (bind _outactors (Actor|GetAllActorsOfClass "/Script/DroidDefense.C_MapMngr"))
  (if (== (Utilities|Array|Length _outactors) 1)
    ;[1 1 1] Find the path
    (bind (_validpathcreated _returnvalue) (Class|CMapMngr|PathFind (Utilities|Array|Get(acopy) _outactors) _x _y (Variables|Default|Getm_TargetX) (Variables|Default|Getm_TargetY) (Variables|Default|GetNodes)))
    (bind _output_get (Variables|Default|SetNodes _returnvalue))
    (for _array_element_2 _output_get
      (Utilities|SpawnPathObject _array_element_2))
    (return _validpathcreated)
    (else
      (return false))))

(fn ClearOldPath
  (Variables|Default|Setm_CurrentNode 0)
  ;[1 1 1] Remove nodes from the old array
  (for (_array_element _array_index) (Variables|Default|Getmrp_PathNodes)
    (Actor|DestroyActor _array_element)
    (Utilities|Array|SetArrayElem (Variables|Default|Getmrp_PathNodes) _array_index 0))
  (Utilities|Array|Clear (Variables|Default|Getmrp_PathNodes))
  (Utilities|Array|Clear (Variables|Default|GetNodes)))