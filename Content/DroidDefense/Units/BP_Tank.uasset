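; BP_Tank is a droid defense unit that drives toward a target location and fires on it, awarding parts to the player when destroyed.
; It spawns its own controller, then uses a simple move to its target every tick.
; When within range, it spawns a BP_GunBullet about once a second, aimed at the target with a yaw offset.
; DealDamage reduces health and, at zero, gives parts to BP_PlayerChar before destroying the tank.
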(event EventBeginPlay
  (Pawn|SpawnDefaultController)
  (Variables|Default|Setm_Health 5e+01)
  (Variables|Default|Setm_PartsDeath 5))

(event Collision|EventActorBeginOverlap
  (params (OtherActor :type Actor%20Object%20Reference)))

(event EventTick
  (params (DeltaSeconds :type Float%20%28single-precision%29))
  (bind _capsulecomponent (Variables|Default|GetCapsuleComponent))
  (bind _m_targetloc (Variables|Default|Getm_TargetLoc))
  (bind _returnvalue (Transformation|GetWorldTransform _capsulecomponent))
  (bind _returnvalue_2 (Math|Rotator|FindLookatRotation (.location _returnvalue) _m_targetloc))
  (Variables|Default|Settimer (+ DeltaSeconds (Variables|Default|Gettimer)))
  (AI|Navigation|SimpleMovetoLocation (Pawn|GetController) (Variables|Default|Getm_TargetLoc))
  (if (and (<= (Math|Vector|VectorLength (- (Transformation|GetActorLocation) (Variables|Default|Getm_TargetLoc))) 5e+02) (>= (Variables|Default|Gettimer) 1.0))
    (Game|SpawnActorfromClass "/Game/DroidDefense/Ammo/BP_GunBullet.BP_GunBullet_C" (Math|Transform|MakeTransform (.location _returnvalue) (Math|Rotator|MakeRotator (.roll _returnvalue_2) (.pitch _returnvalue_2) (- (.yaw _returnvalue_2) 9e+01)) "1,1,1") "Undefined" 0 1.2 0)
    (Variables|Default|Settimer 0.0)))

(event EventDealDamage
  (params (Amount :type Float%20%28single-precision%29))
  (bind _output_get (Variables|Default|Setm_Health (- (Variables|Default|Getm_Health) Amount)))
  (if (<= _output_get 0.0)
    (bind _asbp_player_char (Utilities|Casting|CastToBP_PlayerChar (Game|GetPlayerCharacter 0))
      (:then
        (Default|AddParts _asbp_player_char (Variables|Default|Getm_PartsDeath))
        (Actor|DestroyActor))
      (:CastFailed
        (Actor|DestroyActor)))))

(fn ConstructionScript)