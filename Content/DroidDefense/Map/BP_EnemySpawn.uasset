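; Enemy spawner for Droid Defense that defines the attack waves and spawns their units.
; CreateWaves fills MrWaves with five escalating waves of droids, heavy units and tanks, but this Blueprint's graphs do not advance them.
; SpawnUnit spawns the requested AI type at the actor's location and tracks it in Units, which Tick prunes of invalid entries.
; GetCurrentWave supplies progress text, and AllUnitsGone reports when all waves and units are finished.
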(event EventBeginPlay)

(event Collision|EventActorBeginOverlap
  (params (OtherActor :type Actor%20Object%20Reference)))

(event EventCreateWaves
  (Utilities|Array|Add (Variables|Default|Getmr_Waves) (Utilities|Struct|MakeWave (Utilities|Array|MakeArray (Utilities|Struct|MakeUnitSpawnOrder "BasicUnit" 5 0 1.0)) 0 0.0 12.0))
  (Utilities|Array|Add (Variables|Default|Getmr_Waves) (Utilities|Struct|MakeWave (Utilities|Array|MakeArray (Utilities|Struct|MakeUnitSpawnOrder "BasicUnit" 10 0 0.8) (Utilities|Struct|MakeUnitSpawnOrder "HeavyUnit" 5 0 1.2)) 0 0.0 12.0))
  (Utilities|Array|Add (Variables|Default|Getmr_Waves) (Utilities|Struct|MakeWave (Utilities|Array|MakeArray (Utilities|Struct|MakeUnitSpawnOrder "BasicUnit" 15 0 0.5) (Utilities|Struct|MakeUnitSpawnOrder "HeavyUnit" 10 0 0.9)) 0 0.0 12.0))
  (Utilities|Array|Add (Variables|Default|Getmr_Waves) (Utilities|Struct|MakeWave (Utilities|Array|MakeArray (Utilities|Struct|MakeUnitSpawnOrder "BasicTank" 2 0 5.0)) 0 0.0 12.0))
  (Utilities|Array|Add (Variables|Default|Getmr_Waves) (Utilities|Struct|MakeWave (Utilities|Array|MakeArray (Utilities|Struct|MakeUnitSpawnOrder "BasicUnit" 15 0 0.25) (Utilities|Struct|MakeUnitSpawnOrder "HeavyUnit" 10 0 0.35) (Utilities|Struct|MakeUnitSpawnOrder "BasicUnit" 20 0 0.25)) 0 0.0)))

(event EventTick
  (params (DeltaSeconds :type Float%20%28single-precision%29))
  (for _array_element (Variables|Default|GetUnits)
    (Utilities|IsValid _array_element
      (:Is%20Not%20Valid
        (Utilities|Array|RemoveItem (Variables|Default|GetUnits) _array_element)))))

(fn ConstructionScript)

(fn SpawnUnit
  (params (a_Type :type EUnitTypes%20Enum :default "BasicUnit"))
  (bind _returnvalue (Transformation|GetActorLocation))
  (switch Utilities|FlowControl|Switch|SwitchonEUnitTypes a_Type
    (:BasicUnit
      (bind _returnvalue_2 (AI|SpawnAIFromClass "/Game/DroidDefense/Units/BP_DroidUnit.BP_DroidUnit_C" 0 _returnvalue "0, 0, 0" false))
      (bind _asc_basic_unit (Utilities|Casting|CastToC_BasicUnit _returnvalue_2)
        (:then
          (Utilities|Array|Add (Variables|Default|GetUnits) _asc_basic_unit))
        (:CastFailed
          _))
      (return _asc_basic_unit))
    (:HeavyUnit
      (bind _returnvalue_3 (AI|SpawnAIFromClass "/Game/DroidDefense/Units/BP_HeavyUnit.BP_HeavyUnit_C" 0 _returnvalue "0, 0, 0" false))
      (bind _asc_basic_unit_2 (Utilities|Casting|CastToC_BasicUnit _returnvalue_3)
        (:then
          (Utilities|Array|Add (Variables|Default|GetUnits) _asc_basic_unit_2))
        (:CastFailed
          _))
      (return _asc_basic_unit_2))
    (:BasicTank
      (bind _returnvalue_4 (AI|SpawnAIFromClass "/Game/DroidDefense/Units/BP_Tank.BP_Tank_C" 0 _returnvalue "0, 0, 0" false))
      (bind _asc_basic_unit_3 (Utilities|Casting|CastToC_BasicUnit _returnvalue_4)
        (:then
          (Utilities|Array|Add (Variables|Default|GetUnits) _asc_basic_unit_3))
        (:CastFailed
          _))
      (return _asc_basic_unit_3))))

(fn GetCurrentWave
  (bind _mr_waves (Variables|Default|Getmr_Waves))
  (bind _m_currentwave (Variables|Default|Getm_CurrentWave))
  (bind _returnvalue (Utilities|Array|Length _mr_waves))
  (bind _returnvalue_2 (+ _m_currentwave 1))
  (if (<= _returnvalue_2 _returnvalue)
    (bind _output_get (LocalVariables|Setmessage (Utilities|String|Append (Utilities|String|ToString(Integer) _returnvalue_2) " of " (Utilities|String|ToString(Integer) _returnvalue))))
    (return (Utilities|Text|ToText(String) _output_get))
    (else
      (bind _output_get_2 (LocalVariables|Setmessage "Final!!!"))
      (return (Utilities|Text|ToText(String) _output_get_2)))))

(fn AllUnitsGone
  (if (>= (Variables|Default|Getm_CurrentWave) (Utilities|Array|Length (Variables|Default|Getmr_Waves)))
    (return (<= (Utilities|Array|Length (Variables|Default|GetUnits)) 0))
    (else
      (return false))))